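; Static turret Blueprint that starts firing bullets once its PawnSensing component first sees a pawn, with per-instance color and sensing settings.
; The construction script applies sight, hearing and vision angle; BeginPlay tints the body through a dynamic material.
; The first sighting stores the target, then a looping timer repeatedly spawns bullets along the spawn point's forward vector.
; Nothing aims at the target or stops the firing.
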(event `self.ReceiveBeginPlay`
  ;[1 1 1] turret material instance editable
  (bind _returnvalue (`KismetMaterialLibrary.CreateDynamicMaterialInstance` "/Game/Materials/M_TurretColor.M_TurretColor"))
  (`MaterialInstanceDynamic.SetVectorParameterValue` _returnvalue "Color" (`self.TurretColor`))
  (`PrimitiveComponent.SetMaterial` (`self.Body`) 0 _returnvalue)
  (`KismetSystemLibrary.PrintString` (`KismetStringLibrary.Conv_ColorToString` (`self.TurretColor`)) true true (struct :`G` 0.66 :`B` 1.0 :`A` 1.0) 10.0))

(event `self.PawnSensing.OnSeePawn`
  (params (Pawn :type "Pawn Object Reference"))
  (`/Engine/EditorBlueprintResources/StandardMacros.DoOnce` false
    (:`Completed`
      (set `self.TargetActor` Pawn)
      ; bullet shooting
      (`KismetSystemLibrary.K2_SetTimerDelegate` (delegate `FireWeapon`) 1.0 true :!label _label)
      (`KismetSystemLibrary.PrintString` "Bullet is Shooting")
      (`KismetSystemLibrary.Delay` 0.2)
      (bind _returnvalue (`|SpawnActorFromClass` "/Game/Blueprint/NewFolder/BP_TurretBullet.BP_TurretBullet_C" (`SceneComponent.K2_GetComponentToWorld` (`self.Bulletspawnpoint`)) "Undefined" "MultiplyWithRoot" self null))
      (bind _asbp_turret_bullet (cast `/Game/Blueprint/NewFolder/BP_TurretBullet` _returnvalue))
      (set `MovementComponent.Velocity` (* (`SceneComponent.GetForwardVector` (`self.Bulletspawnpoint`)) 5000.0) (`/Game/Blueprint/NewFolder/BP_TurretBullet.ProjectileMovement` _asbp_turret_bullet)))))

(event `FireWeapon`
  ; bullet shooting
  (goto _label))

(fn `UserConstructionScript`
  (bind _pawnsensing (`self.PawnSensing`))
  ;[1 1 1] instance editable - radius, threshold and vision
  (set `PawnSensingComponent.SightRadius` (`self.CustomSightRadius`) _pawnsensing)
  (set `PawnSensingComponent.HearingThreshold` (`self.CustomHearingThreshold`) _pawnsensing)
  (`PawnSensingComponent.SetPeripheralVisionAngle` _pawnsensing (`self.CustomVisionAngle`)))