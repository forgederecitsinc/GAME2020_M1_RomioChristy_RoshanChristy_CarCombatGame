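; BP_Turret is a turret actor that turns toward vehicle pawns it sees and fires bullets at them.
; The construction script applies custom sight radius, hearing threshold and vision angle to PawnSensing, and BeginPlay tints the body through a dynamic material instance.
; On seeing a BP_VehicleAdvPawnBase, it snaps its yaw to the target, then spawns BP_TurretBullet at the spawn point after a short delay.
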(event `self.ReceiveBeginPlay`
  ;[1 1 1] turret material instance editable
  (bind _returnvalue (`KismetMaterialLibrary.CreateDynamicMaterialInstance` "/Game/Materials/M_TurretColor.M_TurretColor"))
  (`MaterialInstanceDynamic.SetVectorParameterValue` _returnvalue "Color" (`self.TurretColor`))
  (`PrimitiveComponent.SetMaterial` (`self.Body`) 0 _returnvalue)
  (`KismetSystemLibrary.PrintString` (`KismetStringLibrary.Conv_ColorToString` (`self.TurretColor`)) true true (struct :`G` 0.66 :`B` 1.0 :`A` 1.0) 10.0))

(event `self.PawnSensing.OnSeePawn`
  (params (Pawn :type "Pawn Object Reference"))
  ;[1 1 1] Turn on seeing PAWN
  (cast `/Game/VehicleTemplate/Blueprints/BP_VehicleAdvPawnBase` Pawn)
  (`self.K2_SetActorRotation` (`KismetMathLibrary.MakeRotator` 0.0 0.0 (.yaw (`KismetMathLibrary.FindLookAtRotation` (`self.K2_GetActorLocation`) (`self.K2_GetActorLocation` Pawn)))))
  ; bullet shooting
  (`KismetSystemLibrary.Delay` 0.2)
  (`|SpawnActorFromClass` "/Game/Blueprint/NewFolder/BP_TurretBullet.BP_TurretBullet_C" (`SceneComponent.K2_GetComponentToWorld` (`self.Bulletspawnpoint`)) "Undefined" "MultiplyWithRoot" null null))

(fn `UserConstructionScript`
  (bind _pawnsensing (`self.PawnSensing`))
  ;[1 1 1] instance editable - radius, threshold and vision
  (set `PawnSensingComponent.SightRadius` (`self.CustomSightRadius`) _pawnsensing)
  (set `PawnSensingComponent.HearingThreshold` (`self.CustomHearingThreshold`) _pawnsensing)
  (`PawnSensingComponent.SetPeripheralVisionAngle` _pawnsensing (`self.CustomVisionAngle`)))